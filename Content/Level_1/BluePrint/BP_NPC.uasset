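; Level 1 NPC that shows an interaction prompt and displays a line of intro dialogue.
; Its InteractTrigger reveals a TextRender while BP_ThirdPersonCharacter overlaps it and hides it on exit.
; The Interacted event reaches MainUI through the game mode, fills DialogueText with the first IntroDialogue entry, and hides the dialogue box after a short fixed delay.
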(event OnComponentBeginOverlap(InteractTrigger)
  (params (OverlappedComponent :type Primitive%20Component%20Object%20Reference) (OtherActor :type Actor%20Object%20Reference) (OtherComp :type Primitive%20Component%20Object%20Reference) (OtherBodyIndex :type Integer) (bFromSweep :type Boolean) (SweepResult :type Hit%20Result%20Structure%20%28by%20ref%29))
  (Utilities|Casting|CastToBP_ThirdPersonCharacter OtherActor)
  (Development|SetHiddeninGame (Variables|Default|GetTextRender) false false))

(event OnComponentEndOverlap(InteractTrigger)
  (params (OverlappedComponent :type Primitive%20Component%20Object%20Reference) (OtherActor :type Actor%20Object%20Reference) (OtherComp :type Primitive%20Component%20Object%20Reference) (OtherBodyIndex :type Integer))
  (Utilities|Casting|CastToBP_ThirdPersonCharacter OtherActor)
  (Development|SetHiddeninGame (Variables|Default|GetTextRender) true false))

(event EventInteracted
  (bind _asbp_third_person_game_mode (Utilities|Casting|CastToBP_ThirdPersonGameMode (Game|GetGameMode)))
  (Rendering|Components|TextRender|SetText (Variables|/Game/Level_1/UMG/UMG_MainUI.UMG_MainUI_C|GetDialogue_Text (Variables|/Game/ThirdPerson/Blueprints/BP_ThirdPersonGameMode.BP_ThirdPersonGameMode_C|GetMainUI _asbp_third_person_game_mode)) (Utilities|Array|Get(acopy) (Variables|/Game/Level_1/Dialogue/BP_DA_Dialogue.BP_DA_Dialogue_C|GetIntro_Dialogue (Variables|Default|GetText))))
  (Widget|SetVisibility (Variables|/Game/Level_1/UMG/UMG_MainUI.UMG_MainUI_C|GetDialogue_Box (Variables|/Game/ThirdPerson/Blueprints/BP_ThirdPersonGameMode.BP_ThirdPersonGameMode_C|GetMainUI _asbp_third_person_game_mode)) "Visible")
  (Utilities|FlowControl|Delay 3.0)
  (Widget|SetVisibility (Variables|/Game/Level_1/UMG/UMG_MainUI.UMG_MainUI_C|GetDialogue_Box (Variables|/Game/ThirdPerson/Blueprints/BP_ThirdPersonGameMode.BP_ThirdPersonGameMode_C|GetMainUI _asbp_third_person_game_mode)) "Hidden"))

(fn ConstructionScript)