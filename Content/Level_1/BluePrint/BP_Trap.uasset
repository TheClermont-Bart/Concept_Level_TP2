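; BP_Trap is a trigger that opens a referenced door for the player character and closes it gradually once they leave.
; Entering InteractTrigger snaps the door's Cube to a raised position, plays a secret-door sound and resets the step counter.
; Leaving starts LoopIteration, a self-rescheduling timer event that lowers the door in small fixed steps until the counter hits its limit.
; Re-entry does not clear a pending timer.
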(event OnComponentBeginOverlap(InteractTrigger)
  (params (OverlappedComponent :type Primitive%20Component%20Object%20Reference) (OtherActor :type Actor%20Object%20Reference) (OtherComp :type Primitive%20Component%20Object%20Reference) (OtherBodyIndex :type Integer) (bFromSweep :type Boolean) (SweepResult :type Hit%20Result%20Structure%20%28by%20ref%29))
  ;[0.15 0.15 0.15 0.5] Overlap
  (Utilities|Casting|CastToBP_ThirdPersonCharacter OtherActor)
  (Transformation|SetRelativeLocation (Variables|/Game/Level_1/BluePrint/BP_Door_0.BP_Door_0_C|GetCube (Variables|Default|GetDoorReference)) "0.000000,0.000000,200.000000" false false)
  (Audio|SpawnSound2D "/Game/Level_1/Sounds/Zelda_Secret_Door_Opening__Sound_Effect_.Zelda_Secret_Door_Opening__Sound_Effect_" 1.0 1.0 0.0 0)
  (Variables|Default|SetCurrentIndex 0))

(event OnComponentEndOverlap(InteractTrigger)
  (params (OverlappedComponent :type Primitive%20Component%20Object%20Reference) (OtherActor :type Actor%20Object%20Reference) (OtherComp :type Primitive%20Component%20Object%20Reference) (OtherBodyIndex :type Integer))
  ;[0.15 0.15 0.15 0.5] Overlap
  (Utilities|Casting|CastToBP_ThirdPersonCharacter OtherActor)
  (CallFunction|LoopIteration))

(event Custom|LoopIteration
  (bind _doorreference (Variables|Default|GetDoorReference))
  (bind _cube (Variables|/Game/Level_1/BluePrint/BP_Door_0.BP_Door_0_C|GetCube _doorreference))
  ;[0.15 0.15 0.15 0.5] Fermeture de porte
  (Transformation|SetRelativeLocation _cube (- (Variables|/Script/Engine.SceneComponent|GetRelativeLocation _cube) "0.000000,0.000000,10.000000") false false)
  (bind _result (Math|Integer|IncrementInt (Variables|Default|GetCurrentIndex))
    (:%20%20
      (bind _output_get (Variables|Default|SetCurrentIndex _result))
      (if (< _output_get 18)
        (Utilities|Time|SetTimerbyEvent (delegate Custom|LoopIteration) 0.8)))))

(fn ConstructionScript
  (|CallParentFunction))