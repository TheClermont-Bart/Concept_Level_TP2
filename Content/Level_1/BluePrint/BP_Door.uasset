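; BP_Door is a locked door that the player can open and close only while holding a key.
; InteractTrigger overlaps track whether a BP_ThirdPersonCharacter is close and store a reference to it.
; When nearby, the Open_Door event checks the character's HasKey, then a FlipFlop snaps the Cube between raised and original relative positions without animation.
; Without the key, it prints a French missing-key message.
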(event OnComponentBeginOverlap(InteractTrigger)
  (params (OverlappedComponent :type Primitive%20Component%20Object%20Reference) (OtherActor :type Actor%20Object%20Reference) (OtherComp :type Primitive%20Component%20Object%20Reference) (OtherBodyIndex :type Integer) (bFromSweep :type Boolean) (SweepResult :type Hit%20Result%20Structure%20%28by%20ref%29))
  (bind _asbp_third_person_character (Utilities|Casting|CastToBP_ThirdPersonCharacter OtherActor))
  (Variables|Default|SetPlayerRef _asbp_third_person_character)
  (Variables|Default|Setis_player_close true))

(event OnComponentEndOverlap(InteractTrigger)
  (params (OverlappedComponent :type Primitive%20Component%20Object%20Reference) (OtherActor :type Actor%20Object%20Reference) (OtherComp :type Primitive%20Component%20Object%20Reference) (OtherBodyIndex :type Integer))
  (Utilities|Casting|CastToBP_ThirdPersonCharacter OtherActor)
  (Variables|Default|Setis_player_close false)
  (Variables|Default|SetPlayerRef 0))

(event Custom|Open_Door
  (bind _cube (Variables|Default|GetCube))
  (if (Variables|Default|Getis_player_close)
    (if (Variables|/Game/ThirdPerson/Blueprints/BP_ThirdPersonCharacter.BP_ThirdPersonCharacter_C|GetHasKey (Variables|Default|GetPlayerRef))
      (Utilities|FlowControl|FlipFlop
        (:A
          (Transformation|SetRelativeLocation _cube "0.000000,0.000000,200.000000" false false))
        (:B
          (Transformation|SetRelativeLocation _cube "0, 0, 0" false false)))
      (else
        (Development|PrintText "Ta pas la clee")))))

(fn ConstructionScript
  (|CallParentFunction))